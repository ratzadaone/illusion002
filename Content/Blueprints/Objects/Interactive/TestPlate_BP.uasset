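; TestPlate_BP is an interactive weight plate that makes the player's BP_CustomMove_TopDown character explode once a mass threshold is reached.
; A Box overlap starts a looping one-second timer running CalculateMass, which pauses when the box is empty.
; Each tick adds a fixed mass for that character class or static mesh mass for other overlapping actors.
; TotalMass is never reset, so it accumulates across ticks.
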(event `self.ReceiveBeginPlay`)

(event `self.Box.OnComponentBeginOverlap`
  (params (OverlappedComponent :type "PrimitiveComponent Object Reference") (OtherActor :type "Actor Object Reference") (OtherComp :type "PrimitiveComponent Object Reference") (OtherBodyIndex :type Integer) (bFromSweep :type Boolean) (SweepResult :type "HitResult Structure (by ref)"))
  (`self.GetTotalMass`))

(event `GetTotalMass`
  (`KismetSystemLibrary.K2_SetTimer` null "CalculateMass" 1.0 true))

(fn `CalculateMass`
  (locals (TotalMass :type "Float (double-precision)"))
  (bind _overlappingactors (`PrimitiveComponent.GetOverlappingActors` (`self.Box`) null))
  (if (> (`KismetArrayLibrary.Array_Length` _overlappingactors) 0)
    (for _array_element _overlappingactors
      (if (`.bSuccess` (cast `/Game/Blueprints/Player/BP_CustomMove_TopDown` _array_element :!pure true))
        (set `local.TotalMass` (+ (`local.TotalMass`) 55.0))
        (else
          (set `local.TotalMass` (+ (`local.TotalMass`) (`PrimitiveComponent.GetMass` (`self.GetComponentByClass` _array_element "/Script/Engine.StaticMeshComponent"))))))
      (if (>= (`local.TotalMass`) 90.0)
        (`/Game/Blueprints/Player/BP_CustomMove_TopDown.Explode` (cast `/Game/Blueprints/Player/BP_CustomMove_TopDown` (`GameplayStatics.GetPlayerCharacter` 0) :!pure true))))
    (else
      (`KismetSystemLibrary.K2_PauseTimer` null "CalculateMass"))))

(fn `UserConstructionScript`)