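; TestLever_BP is an interactive lever that operates a bridge when pulled.
; The use interface event flip-flops a timeline forward and back to swing the lever mesh's pitch.
; When the forward throw finishes, it sends a use interface message to the first BP_Bridge found in the level; the return throw sends none.
; The overlap interface event shows or hides the key prompt on the player controller's main UI.
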(event `self.ReceiveBeginPlay`
  (set `self.PlayerControllerRef` (cast `/Game/Blueprints/Player/BP_TopDownController` (`GameplayStatics.GetPlayerController` 0) :!pure true)))

(event `/Game/Blueprints/Interface/InteractInterface.Interface_Use`
  (bind _isa (`/Engine/EditorBlueprintResources/StandardMacros.FlipFlop`)
    (:`A`
      (bind (_direction _newtrack_0) (`Timeline|Timeline_0` :!label _label)
        (:`Update`
          (`SceneComponent.K2_SetRelativeRotation` (`self.StaticMesh1`) (`KismetMathLibrary.MakeRotator` 0.0 (`KismetMathLibrary.Lerp` -45.0 45.0 _newtrack_0)) false false))
        (:`Finished`
          (if _isa
            (bind _outactors (`GameplayStatics.GetAllActorsOfClass` "/Game/Blueprints/Objects/BP_Bridge.BP_Bridge_C"))
            (message `/Game/Blueprints/Interface/InteractInterface.Interface_Use` (`|GetArrayItem` _outactors))))))
    (:`B`
      (goto _label :!via `Reverse`))))

(event `/Game/Blueprints/Interface/InteractInterface.Interface_Overlap`
  (params (StartTrueEndFalse :type Boolean))
  (bind _w_mainui_ref (`/Game/Blueprints/Player/BP_TopDownController.W_MainUI_Ref` (`self.PlayerControllerRef`)))
  (bind _instructiontext (`/Game/Blueprints/UI/W_MainUI.InstructionText` _w_mainui_ref))
  (if StartTrueEndFalse
    (`TextBlock.SetText` (`/Game/Blueprints/UI/W_MainUI.DYnamicText` _w_mainui_ref) "Press \"E\" To Operate")
    (`Widget.SetVisibility` _instructiontext "HitTestInvisible")
    (else
      (`Widget.SetVisibility` _instructiontext "Hidden"))))

(fn `UserConstructionScript`)