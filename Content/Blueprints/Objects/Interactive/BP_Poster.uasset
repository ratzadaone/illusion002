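; BP_Poster is an interactive poster that the player collects with the E key prompt shown on overlap.
; The construction script applies the texture for its PosterNr from the PostersDataList table to a dynamic material.
; Use increments the player controller's PostersCollected, updates the main UI, rebuilds the material and animates its Offset through a timeline.
; The actor stays after collection, as DestroyActor is unwired, and Use has no repeat guard.
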(event `/Game/Blueprints/Interface/InteractInterface.Interface_Overlap`
  (params (StartTrueEndFalse :type Boolean))
  (bind _w_mainui_ref (`/Game/Blueprints/Player/BP_TopDownController.W_MainUI_Ref` (`self.PlayerController_Ref`)))
  (bind _instructiontext (`/Game/Blueprints/UI/W_MainUI.InstructionText` _w_mainui_ref))
  (if StartTrueEndFalse
    (`TextBlock.SetText` (`/Game/Blueprints/UI/W_MainUI.DYnamicText` _w_mainui_ref) "Press \"E\" To Collect Poster")
    (`Widget.SetVisibility` _instructiontext "HitTestInvisible")
    (else
      (`Widget.SetVisibility` _instructiontext "Hidden"))))

(event `/Game/Blueprints/Interface/InteractInterface.Interface_Use`
  (bind _playercontroller_ref (`self.PlayerController_Ref`))
  (bind _result (`/Engine/EditorBlueprintResources/StandardMacros.IncrementInt` (`/Game/Blueprints/Player/BP_TopDownController.PostersCollected` _playercontroller_ref))
    (:`  `
      (bind _output_get (set `/Game/Blueprints/Player/BP_TopDownController.PostersCollected` _result _playercontroller_ref))
      (`TextBlock.SetText` (`/Game/Blueprints/UI/W_MainUI.PostersCollected` (`/Game/Blueprints/Player/BP_TopDownController.W_MainUI_Ref` _playercontroller_ref)) (`KismetTextLibrary.Conv_IntToText` _output_get))
      (bind _returnvalue (`PrimitiveComponent.CreateDynamicMaterialInstance` (`self.PlaneMesh`) 0 "/Game/Materials/Poster.Poster"))
      (bind _returnvalue_2 (`|GetDataTableRow` "/Game/Blueprints/Enums/PostersDataList.PostersDataList" (`KismetStringLibrary.Conv_StringToName` (`|GetEnumeratorNameAsString` (`self.PosterNr`))))
        (:`then`
          (`MaterialInstanceDynamic.SetTextureParameterValue` _returnvalue "PosterTexture" (`.PosterImage_5_FA0F09564896A033D0AFED8375C0023C` (break `/Game/Blueprints/Enums/Posters_list` _returnvalue_2)))
          (bind (_direction _newtrack_1) (`Timeline|Timeline_0`)
            (:`Update`
              (`MaterialInstanceDynamic.SetScalarParameterValue` _returnvalue "Offset" _newtrack_1)
              (`KismetSystemLibrary.PrintString` (`KismetStringLibrary.Conv_DoubleToString` _newtrack_1)))))))))

(event `self.ReceiveBeginPlay`
  (set `self.PlayerController_Ref` (cast `/Game/Blueprints/Player/BP_TopDownController` (`GameplayStatics.GetPlayerController` 0) :!pure true)))

(fn `UserConstructionScript`
  (bind _returnvalue (`|GetDataTableRow` "/Game/Blueprints/Enums/PostersDataList.PostersDataList" (`KismetStringLibrary.Conv_StringToName` (`|GetEnumeratorNameAsString` (`self.PosterNr`))))
    (:`then`
      (bind _returnvalue_2 (`PrimitiveComponent.CreateDynamicMaterialInstance` (`self.PlaneMesh`) 0 "/Game/Materials/Poster.Poster"))
      (`MaterialInstanceDynamic.SetTextureParameterValue` _returnvalue_2 "PosterTexture" (`.PosterImage_5_FA0F09564896A033D0AFED8375C0023C` (break `/Game/Blueprints/Enums/Posters_list` _returnvalue))))))